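; Spawner actor that builds a chain of BP_Tunnel segments and populates it with pickups and enemies.
; On BeginPlay it clears existing tunnels, health packs and enemies, then lays an initial run starting at the player pawn.
; Each later segment attaches at the newest tunnel's SpawnPoint, receives a spawner reference and is randomized by color index.
; Each attached segment also spawns either a health pack or, more often, an enemy at a random offset.
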(event `self.ReceiveBeginPlay`
  (`self.SpawnInitialTunnels`))

(fn `SpawnEnemy`
  (params (Location :type "Vector Structure"))
  (`|SpawnActorFromClass` "/Game/InfiniteMatrix/Blueprints/BP_Enemy.BP_Enemy_C" (`KismetMathLibrary.MakeTransform` (`KismetMathLibrary.MakeVector` (- (.x Location) (`KismetMathLibrary.RandomFloatInRange` 500.0 1500.0)) (`KismetMathLibrary.RandomFloatInRange` -100.0 100.0) (`KismetMathLibrary.RandomFloatInRange` -100.0 100.0))) "Undefined" "MultiplyWithRoot" null null))

(fn `SpawnHealthPack`
  (params (`Spawn Transform Location` :type "Vector Structure"))
  (`|SpawnActorFromClass` "/Game/InfiniteMatrix/Blueprints/BP_HealthPack.BP_HealthPack_C" (`KismetMathLibrary.MakeTransform` (`KismetMathLibrary.MakeVector` (- (.x `Spawn Transform Location`) (`KismetMathLibrary.RandomFloatInRange` 500.0 1500.0)) (`KismetMathLibrary.RandomFloatInRange` -300.0 300.0) (`KismetMathLibrary.RandomFloatInRange` -300.0 300.0))) "Undefined" "MultiplyWithRoot" null null))

(fn `SpawnInitialTunnels`
  (`|ExecutionSequence`
    (:`then_0`
      (bind _outactors (`GameplayStatics.GetAllActorsOfClass` "/Game/InfiniteMatrix/Blueprints/BP_Tunnel.BP_Tunnel_C"))
      (for _array_element _outactors
        (`self.K2_DestroyActor` _array_element)))
    (:`then_1`
      (bind _outactors_2 (`GameplayStatics.GetAllActorsOfClass` "/Game/InfiniteMatrix/Blueprints/BP_HealthPack.BP_HealthPack_C"))
      (for _array_element_2 _outactors_2
        (`self.K2_DestroyActor` _array_element_2)))
    (:`then_2`
      (bind _outactors_3 (`GameplayStatics.GetAllActorsOfClass` "/Game/InfiniteMatrix/Blueprints/BP_Enemy.BP_Enemy_C"))
      (for _array_element_3 _outactors_3
        (`self.K2_DestroyActor` _array_element_3)))
    (:`then_3`
      (for _ (range 11)
        (`/Engine/EditorBlueprintResources/StandardMacros.IsValid` (`self.NewestTunnel`)
          (:`Is Valid`
            (`self.SpawnTunnelAtSpawnPoint` 0))
          (:`Is Not Valid`
            (`self.SpawnTunnel` (`self.K2_GetActorLocation` (`GameplayStatics.GetPlayerPawn` 0)))))))))

(fn `SpawnTunnel`
  (params (SpawnLocation :type "Vector Structure") (ColorIndex :type Integer))
  (locals (NewLocalVar :type "/Game/InfiniteMatrix/Blueprints/BP_TunnelSpawner Object Reference") (BPPlayer :type "/Game/InfiniteMatrix/Blueprints/BP_Player Object Reference"))
  (bind _returnvalue (`|SpawnActorFromClass` "/Game/InfiniteMatrix/Blueprints/BP_Tunnel.BP_Tunnel_C" (`KismetMathLibrary.MakeTransform` SpawnLocation) "Undefined" "MultiplyWithRoot" null null))
  (bind _output_get (set `self.NewestTunnel` _returnvalue))
  (set `/Game/InfiniteMatrix/Blueprints/BP_Tunnel.TunnelSpawner` self _output_get)
  (`/Game/InfiniteMatrix/Blueprints/BP_Tunnel.RandomizeWall` _output_get ColorIndex)
  (`/Game/InfiniteMatrix/Blueprints/BP_Tunnel.RandomizeTunnel` _returnvalue ColorIndex))

(fn `SpawnTunnelAtSpawnPoint`
  (params (ColorIndex :type Integer))
  (bind _returnvalue (`SceneComponent.K2_GetComponentLocation` (`/Game/InfiniteMatrix/Blueprints/BP_Tunnel.SpawnPoint` (`self.NewestTunnel`))))
  (`self.SpawnTunnel` _returnvalue ColorIndex)
  (if (== (`KismetMathLibrary.RandomInteger` 3) 2)
    (`self.SpawnHealthPack` _returnvalue)
    (else
      (`self.SpawnEnemy` _returnvalue))))

(fn `UserConstructionScript`)