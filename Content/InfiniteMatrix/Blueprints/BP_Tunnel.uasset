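; BP_Tunnel is a tunnel segment with a spinning holed wall obstacle, used in endlessly spawned tunnels.
; Passing its trigger adds score, updates the player's stage bar, has TunnelSpawner spawn the next tunnel in the player's color, then destroys the segment.
; Hitting the wall damages the player, deducts score, sets the death flag and disables wall collision.
; Randomize functions set the wall's mesh and roll, plus color-indexed wall and tunnel materials.
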(event `self.ReceiveTick`
  (params (DeltaSeconds :type "Float (single-precision)"))
  (`SceneComponent.K2_AddLocalRotation` (`self.WallMesh`) (`KismetMathLibrary.MakeRotator` (* DeltaSeconds (`self.RotateSpeed`))) false false))

(event `self.TriggerZone.OnComponentBeginOverlap`
  (params (OverlappedComponent :type "PrimitiveComponent Object Reference") (OtherActor :type "Actor Object Reference") (OtherComp :type "PrimitiveComponent Object Reference") (OtherBodyIndex :type Integer) (bFromSweep :type Boolean) (SweepResult :type "HitResult Structure (by ref)"))
  (bind _asbp_player (cast `/Game/InfiniteMatrix/Blueprints/BP_Player` OtherActor))
  (`/Game/InfiniteMatrix/Blueprints/BP_Player.IncrementScore` _asbp_player 1)
  (`/Game/InfiniteMatrix/Blueprints/BP_Player.UpdateStageBar` _asbp_player (`/Game/InfiniteMatrix/Blueprints/BP_Player.Score` _asbp_player) 0)
  (`/Game/InfiniteMatrix/Blueprints/BP_TunnelSpawner.SpawnTunnelAtSpawnPoint` (`self.TunnelSpawner`) (`/Game/InfiniteMatrix/Blueprints/BP_Player.ColorIndex` _asbp_player))
  (`self.K2_DestroyActor`))

(event `self.WallMesh.OnComponentHit`
  (params (HitComponent :type "PrimitiveComponent Object Reference") (OtherActor :type "Actor Object Reference") (OtherComp :type "PrimitiveComponent Object Reference") (NormalImpulse :type "Vector Structure") (Hit :type "HitResult Structure (by ref)"))
  (bind _asbp_player (cast `/Game/InfiniteMatrix/Blueprints/BP_Player` OtherActor))
  (`GameplayStatics.ApplyDamage` _asbp_player 25.0)
  (`GameplayStatics.PlaySound2D` "/Game/Interface_And_Item_Sounds/WAV/Error_Buzz_02.Error_Buzz_02" 1.0 1.0 0.0 null null)
  (`PrimitiveComponent.SetCollisionEnabled` HitComponent "NoCollision")
  (set `/Game/InfiniteMatrix/Blueprints/BP_Player.IsDead` (<= (`/Game/InfiniteMatrix/Blueprints/BP_Player.CurrentHealth` _asbp_player) 0.0) _asbp_player)
  (`/Game/InfiniteMatrix/Blueprints/BP_Player.IncrementScore` _asbp_player -1))

(fn `RandomizeTunnel`
  (params (Index :type Integer))
  (`PrimitiveComponent.SetMaterial` (`self.StaticMeshComponent`) 0 (select `int` Index :`0` "/Game/InfiniteMatrix/Materials/MI_Tunnel.MI_Tunnel" :`1` "/Game/InfiniteMatrix/Materials/MI_Tunnel1_Blue.MI_Tunnel1_Blue" :`2` "/Game/InfiniteMatrix/Materials/MI_Tunnel1_Purple.MI_Tunnel1_Purple" :`3` "/Game/InfiniteMatrix/Materials/MI_Tunnel_Red.MI_Tunnel_Red" :!type "MaterialInterface Object Reference")))

(fn `RandomizeWall`
  (params (ColorIndex :type Integer))
  (bind _wallmesh (`self.WallMesh`))
  (`StaticMeshComponent.SetStaticMesh` _wallmesh (select `int` (`KismetMathLibrary.RandomIntegerInRange` 0 3) :`0` "/Game/InfiniteMatrix/Meshes/SM_Hole_01.SM_Hole_01" :`1` "/Game/InfiniteMatrix/Meshes/SM_Hole_02.SM_Hole_02" :`2` "/Game/InfiniteMatrix/Meshes/SM_Hole_03.SM_Hole_03" :`3` "/Game/InfiniteMatrix/Meshes/SM_Hole_04.SM_Hole_04" :!type "StaticMesh Object Reference"))
  (`SceneComponent.K2_AddLocalRotation` (`self.WallMesh`) (`KismetMathLibrary.MakeRotator` (`KismetMathLibrary.RandomFloatInRange` 0.0 360.0)) false false)
  (`PrimitiveComponent.SetMaterial` _wallmesh 0 (select `int` ColorIndex :`0` "/Game/InfiniteMatrix/Materials/MI_Hole.MI_Hole" :`1` "/Game/InfiniteMatrix/Materials/MI_Hole_Blue.MI_Hole_Blue" :`2` "/Game/InfiniteMatrix/Materials/MI_Hole_Purple.MI_Hole_Purple" :`3` "/Game/InfiniteMatrix/Materials/MI_Hole_Red.MI_Hole_Red" :!type "MaterialInterface Object Reference")))

(fn `UserConstructionScript`)