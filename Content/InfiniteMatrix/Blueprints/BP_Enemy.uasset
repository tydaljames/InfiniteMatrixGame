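; BP_Enemy is an enemy actor that damages the player on contact and can be killed by the player's projectiles.
; Any hit on its Sphere destroys it: a player hit plays a buzz and applies damage, while a projectile hit increments kills, updates the stage bar and plays a click.
; A player overlapping its TriggerZone also destroys it, with no damage, score or sound.
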(event `self.Sphere.OnComponentHit`
  (params (HitComponent :type "PrimitiveComponent Object Reference") (OtherActor :type "Actor Object Reference") (OtherComp :type "PrimitiveComponent Object Reference") (NormalImpulse :type "Vector Structure") (Hit :type "HitResult Structure (by ref)"))
  (`self.K2_DestroyActor`)
  (bind _asbp_player (cast `/Game/InfiniteMatrix/Blueprints/BP_Player` OtherActor)
    (:`then`
      (`GameplayStatics.PlaySound2D` "/Game/Interface_And_Item_Sounds/WAV/Error_Buzz_02.Error_Buzz_02" 1.0 1.0 0.0 null null)
      (`GameplayStatics.ApplyDamage` _asbp_player 20.0))
    (:`CastFailed`
      (cast `/Game/InfiniteMatrix/Blueprints/BP_FirstPersonProjectile` OtherActor)
      (bind _asbp_player_2 (cast `/Game/InfiniteMatrix/Blueprints/BP_Player` (`GameplayStatics.GetPlayerPawn` 0)))
      (`/Game/InfiniteMatrix/Blueprints/BP_Player.IncrementKills` _asbp_player_2 1)
      (`/Game/InfiniteMatrix/Blueprints/BP_Player.UpdateStageBar` _asbp_player_2 (`/Game/InfiniteMatrix/Blueprints/BP_Player.Score` _asbp_player_2) 0)
      (`GameplayStatics.PlaySound2D` "/Game/Interface_And_Item_Sounds/WAV/Flick_Switch_01.Flick_Switch_01" 1.0 1.0 0.0 null null))))

(event `self.TriggerZone.OnComponentBeginOverlap`
  (params (OverlappedComponent :type "PrimitiveComponent Object Reference") (OtherActor :type "Actor Object Reference") (OtherComp :type "PrimitiveComponent Object Reference") (OtherBodyIndex :type Integer) (bFromSweep :type Boolean) (SweepResult :type "HitResult Structure (by ref)"))
  (cast `/Game/InfiniteMatrix/Blueprints/BP_Player` OtherActor)
  (`self.K2_DestroyActor`))

(fn `UserConstructionScript`)